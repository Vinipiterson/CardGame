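; BP_Cg_PreviewMesh is a card game preview actor that follows a given screen position in the world.
; Its UpdatePosition event, when the actor is not hidden, deprojects that position through player controller 0 and runs a long Visibility line trace.
; The actor moves to the hit location without checking that the trace hit anything.
; Debug output remains: a position print on every call and a timed trace drawing.
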(event Custom|UpdatePosition
  (params (ScreenPosition :type Vector%202D%20Structure%20%28by%20ref%29))
  (bind _returnvalue (Game|GetPlayerController 0))
  (bind (_worldposition _worlddirection) (Class|GameplayStatics|DeprojectScreentoWorld _returnvalue ScreenPosition))
  (Development|PrintString (Utilities|String|ToString(Vector2d) ScreenPosition))
  (if (not (Variables|Rendering|GetbHidden))
    (bind _outhit (Collision|LineTraceByChannel _worldposition (+ _worldposition (* _worlddirection 1e+04)) "TraceTypeQuery1" false 0 "ForDuration"))
    (Transformation|SetActorLocation (.Location (Collision|BreakHitResult _outhit)) false false)))

(fn ConstructionScript)