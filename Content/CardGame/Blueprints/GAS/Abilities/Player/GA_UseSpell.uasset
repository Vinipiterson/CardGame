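; Gameplay ability that plays the player's current card as a spell at a targeted location.
; After committing, it waits for target data, applies the card's damage effect to the owner to set the damage attribute, then discards the card.
; With authority, it spawns the card's spell actors above the target, passing each the card definition, team tag and an outgoing damage effect spec.
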(event Ability|EventActivateAbility
  (bind _returnvalue (Ability|CommitAbility))
  (if _returnvalue
    (bind _datahandle (|GetUseCardTargetData)
      (:ValidData
        (Variables|Default|SetTargetData (Ability|TargetData|GetHitResultfromTargetData _datahandle))
        (bind _asbp_cg_player_state (Utilities|Casting|CastToBP_Cg_PlayerState (Ability|GetOwningActorfromActorInfo))
          (:then
            (bind _output_get (Variables|Default|SetPS _asbp_cg_player_state))
            (Variables|Default|SetCardDefinition (Class|CgPlayerState|GetCurrentCard _output_get))
            (CallFunction|SetDamage)
            (Class|CgPlayerState|DiscardCard (Variables|Default|GetPS))
            (if (Ability|HasAuthority (Ability|GetAvatarActorfromActorInfo))
              (for _index (range 1 (Variables|/Script/CardGame.CgCardData|GetNumToSpawn (.CardData (Utilities|Struct|BreakCgCardDefinition (Variables|Default|GetCardDefinition)))))
                (bind _returnvalue_2 (Class|CgCombatInterface|GetTeamTag(Message) (Ability|GetOwningActorfromActorInfo)))
                (Game|SpawnActorfromClass (Variables|/Script/CardGame.CgCardData|GetSpellClass (.CardData (Utilities|Struct|BreakCgCardDefinition (Variables|Default|GetCardDefinition)))) (CallFunction|GetSpawnTransform) "AlwaysSpawn" "MultiplyWithRoot" (Ability|GetOwningActorfromActorInfo) (Variables|Default|GetCardDefinition) _returnvalue_2 (Ability|MakeOutgoingGameplayEffectSpec "/Game/CardGame/Blueprints/GAS/Effects/GE_Damage.GE_Damage_C") (.AsPawn (Utilities|Casting|CastToPawn (Ability|GetAvatarActorfromActorInfo)))))
              (Ability|EndAbility)
              (else
                (Ability|EndAbility))))
          (:CastFailed
            (Ability|CancelAbility)))))
    (else
      (Ability|CancelAbility))))

(fn GetSpawnTransform
  (return (Math|Transform|MakeTransform (+ (.Location (Collision|BreakHitResult (Variables|Default|GetTargetData))) "0.000000,0.000000,600.000000"))))

(fn SetDamage
  ;[0.15 0.15 0.15 0.5] Set damage attribute on player state
  (Ability|ApplyGameplayEffectSpecToOwner (Ability|MakeOutgoingGameplayEffectSpec (Variables|/Script/CardGame.CgCardData|GetPlayerDamageGameplayEffect (.CardData (Utilities|Struct|BreakCgCardDefinition (Variables|Default|GetCardDefinition)))))))