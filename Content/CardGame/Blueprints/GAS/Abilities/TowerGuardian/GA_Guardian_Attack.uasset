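; Gameplay ability for the card game's tower guardian that fires an arrow at its current combat target.
; On activation it commits, gets the target from the avatar, sets a facing warp target and plays the fire montage.
; An attack gameplay event then triggers a server-only spawn of the arrow from the mesh socket, aimed at the target.
; The arrow carries a damage effect spec, and the ability ends after spawning.
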(event Ability|EventActivateAbility
  (bind _returnvalue (Ability|CommitAbility))
  (if _returnvalue
    (CallFunction|UpdateFacingWarpTarget)
    (Utilities|IsValid (Variables|Default|GetCombatTarget)
      (:Is%20Valid
        (CallFunction|UpdateTeamTag)
        (|PlayMontageandWaitProxy "None" "/Game/Minecraft/Meshes/Skeleton/Animations/AM_Skeleton_Fire.AM_Skeleton_Fire" 1.0 "None" false 1.0 0.0 false
          (:then
            (Ability|Tasks|WaitGameplayEvent "(TagName=\"CardGame.Ability.Event.Attack\")" 0
              (:EventReceived
                (if (Ability|HasAuthority (Ability|GetAvatarActorfromActorInfo))
                  (CallFunction|SpawnProjectile)
                  (Ability|EndAbility)))))))
      (:Is%20Not%20Valid
        (Ability|EndAbility)))))

(fn UpdateFacingWarpTarget
  (bind _returnvalue (Class|CgCombatInterface|GetCombatTarget(Message) (Ability|GetAvatarActorfromActorInfo)))
  (bind _output_get (Variables|Default|SetCombatTarget _returnvalue))
  (Utilities|IsValid _output_get
    (:Is%20Valid
      (Class|CgCombatInterface|SetFacingWarpTargetLocation(Message) (Ability|GetAvatarActorfromActorInfo) (Transformation|GetActorLocation _returnvalue)))))

(fn UpdateTeamTag
  (bind _returnvalue (Class|CgCombatInterface|GetTeamTag(Message) (Ability|GetAvatarActorfromActorInfo)))
  (Variables|Default|SetTeamTag _returnvalue))

(fn SpawnProjectile
  (bind _returnvalue (Ability|GetOwningActorfromActorInfo))
  (Utilities|FlowControl|Sequence
    (:then_0
      (bind _combattarget (Variables|Default|GetCombatTarget)
        (:then
          (bind _output_get (LocalVariables|SetSpawnLocation (Transformation|GetSocketLocation (Actor|GetComponentbyClass (Ability|GetAvatarActorfromActorInfo) "/Script/Engine.SkeletalMeshComponent") "ArrowSpawn")))
          (LocalVariables|SetSpawnRotation (Math|Rotator|FindLookatRotation _output_get (Transformation|GetActorLocation _combattarget))))
        (:else
          (Ability|EndAbility))))
    (:then_1
      (bind _returnvalue_2 (CallFunction|MakeDamageSpec))
      (Game|SpawnActorfromClass "/Game/CardGame/Blueprints/Towers/Guardian/B_Arrow_Guardian.B_Arrow_Guardian_C" (Math|Transform|MakeTransform (LocalVariables|GetSpawnLocation) (LocalVariables|GetSpawnRotation)) "AlwaysSpawn" "MultiplyWithRoot" _returnvalue _returnvalue_2 (.AsPawn (Utilities|Casting|CastToPawn _returnvalue))))))

(fn MakeDamageSpec
  (bind _returnvalue (Ability|GetAbilitySystemComponentfromActorInfo))
  (return (GameplayEffects|MakeOutgoingSpec _returnvalue "/Game/CardGame/Blueprints/GAS/Effects/GE_Damage.GE_Damage_C" 1.0 (GameplayEffects|MakeEffectContext _returnvalue))))