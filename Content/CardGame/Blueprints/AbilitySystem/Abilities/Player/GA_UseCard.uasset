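; Gameplay ability that plays the player's current card, spawning that card's AI units in the world.
; After committing, it reads the card and spawn transform from the player state, then discards the card.
; Only the authority spawns the card's unit count, raising air-terrain units higher than others.
; Each spawned enemy-class unit inherits the owner's team tag; a failed commit or cast cancels the ability.
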(event Ability|EventActivateAbility
  (bind _returnvalue (Ability|CommitAbility))
  (if _returnvalue
    (bind _asbp_cg_player_state (Utilities|Casting|CastToBP_Cg_PlayerState (Ability|GetOwningActorfromActorInfo))
      (:then
        (bind _output_get (Variables|Default|SetPS _asbp_cg_player_state))
        (Variables|Default|SetCardDefinition (Class|CgPlayerState|GetCurrentCard _output_get))
        (Variables|Default|SetSpawnTransform (Class|CgPlayerState|GetSpawnTransform _output_get))
        (Class|CgPlayerState|DiscardCard (Variables|Default|GetPS))
        (if (Ability|HasAuthority (Ability|GetAvatarActorfromActorInfo))
          (for _index (range 1 (Variables|/Script/CardGame.CgCardData|GetNumToSpawn (.CardData (Utilities|Struct|BreakCgCardDefinition (Variables|Default|GetCardDefinition)))))
            (bind _returnvalue_2 (Game|SpawnActorfromClass (Variables|/Script/CardGame.CgCardData|GetAIClass (.CardData (Utilities|Struct|BreakCgCardDefinition (Variables|Default|GetCardDefinition)))) (Math|Transform|MakeTransform (+ (.location (Variables|Default|GetSpawnTransform)) (select (GameplayTags|MatchesTag (Variables|/Script/CardGame.CgCardData|GetTerrainTag (.CardData (Utilities|Struct|BreakCgCardDefinition (Variables|Default|GetCardDefinition)))) "(TagName=\"CardGame.Terrain.Air\")") "0.000000,0.000000,300.000000" "0.000000,0.000000,100.000000")) (.rotation (Variables|Default|GetSpawnTransform)) (.scale (Variables|Default|GetSpawnTransform))) "AdjustIfPossibleButAlwaysSpawn" "MultiplyWithRoot" (Ability|GetOwningActorfromActorInfo) 0))
            (bind _ascg_enemy (Utilities|Casting|CastToCgEnemy _returnvalue_2))
            (bind _returnvalue_3 (Class|CgCombatInterface|GetTeamTag(Message) (Ability|GetOwningActorfromActorInfo)))
            (Variables|/Script/CardGame.CgEnemy|SetTeamTag _ascg_enemy _returnvalue_3))
          (Ability|EndAbility)
          (else
            (Ability|EndAbility))))
      (:CastFailed
        (Ability|CancelAbility)))
    (else
      (Ability|CancelAbility))))