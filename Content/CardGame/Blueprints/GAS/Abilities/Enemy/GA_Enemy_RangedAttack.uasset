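; Gameplay ability for an enemy ranged attack in a card game, driven by the avatar's card definition.
; On activation it commits, sets a facing warp target on the combat target and plays a random attack montage from card data.
; The montage's Attack event triggers a server-only projectile spawn from the card's socket, aimed at the target and carrying a GE_Damage spec.
; A team-filtered ApplyDamage function is defined but never called here.
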(event Ability|EventActivateAbility
  (bind _carddefinition (Variables|Default|GetCardDefinition))
  (bind _carddata (Utilities|Struct|BreakCgCardDefinition _carddefinition))
  (bind _returnvalue (Class|CgCardData|GetRandomAttackMontage _carddata))
  (bind _returnvalue_2 (Ability|CommitAbility))
  (if _returnvalue_2
    (Variables|Default|SetDamageApplied false)
    (CallFunction|UpdateFacingWarpTarget)
    (CallFunction|UpdateTeamTag)
    (CallFunction|UpdateCardDefinition)
    (Utilities|IsValid _returnvalue
      (:Is%20Valid
        (|PlayMontageandWaitProxy "None" _returnvalue 1.0 "None" false 1.0 0.0 false
          (:then
            (Ability|Tasks|WaitGameplayEvent "(TagName=\"CardGame.Ability.Event.Attack\")" 0
              (:EventReceived
                (if (Ability|HasAuthority (Ability|GetAvatarActorfromActorInfo))
                  (CallFunction|SpawnProjectile)))))
          (:OnCompleted
            (Ability|EndAbility :!label _label))
          (:OnInterrupted
            (goto _label))
          (:OnCancelled
            (goto _label)))))))

(fn ApplyDamage
  (params (Target :type Actor%20Object%20Reference))
  (if (Utilities|DoesObjectImplementInterface Target "/Script/CardGame.CgCombatInterface")
    (bind _returnvalue (Class|CgCombatInterface|IsfromTeam(Message) Target (Variables|Default|GetTeamTag)))
    (if (not _returnvalue)
      (if (not (and (Variables|/Script/CardGame.CgCardData|GetbMaleeSingleHit (.CardData (Utilities|Struct|BreakCgCardDefinition (Variables|Default|GetCardDefinition)))) (Variables|Default|GetDamageApplied)))
        (Utilities|IsValid (Ability|GetAbilitySystemComponent Target)
          (:Is%20Valid
            (GameplayEffects|ApplyGameplayEffectSpecToSelf (Ability|GetAbilitySystemComponent Target) (Ability|MakeOutgoingGameplayEffectSpec (Variables|Default|GetDamageGameplayEffect)))
            (Variables|Default|SetDamageApplied true)))))))

(fn UpdateFacingWarpTarget
  (bind _returnvalue (Class|CgCombatInterface|GetCombatTarget(Message) (Ability|GetAvatarActorfromActorInfo)))
  (bind _output_get (Variables|Default|SetCombatTarget _returnvalue))
  (Utilities|IsValid _output_get
    (:Is%20Valid
      (Class|CgCombatInterface|SetFacingWarpTargetLocation(Message) (Ability|GetAvatarActorfromActorInfo) (Transformation|GetActorLocation _returnvalue)))))

(fn UpdateTeamTag
  (bind _returnvalue (Class|CgCombatInterface|GetTeamTag(Message) (Ability|GetAvatarActorfromActorInfo)))
  (Variables|Default|SetTeamTag _returnvalue))

(fn UpdateCardDefinition
  (bind _returnvalue (Class|CgCombatInterface|GetCardDefinition(Message) (Ability|GetAvatarActorfromActorInfo)))
  (Variables|Default|SetCardDefinition _returnvalue))

(fn SpawnProjectile
  (bind _returnvalue (Ability|GetOwningActorfromActorInfo))
  (Utilities|FlowControl|Sequence
    (:then_0
      (bind _output_get (LocalVariables|SetSpawnLocation (Transformation|GetSocketLocation (Actor|GetComponentbyClass (Ability|GetAvatarActorfromActorInfo) "/Script/Engine.SkeletalMeshComponent") (Variables|/Script/CardGame.CgCardData|GetAttackSocketName (.CardData (Utilities|Struct|BreakCgCardDefinition (Variables|Default|GetCardDefinition)))))))
      (LocalVariables|SetSpawnRotation (Math|Rotator|FindLookatRotation _output_get (Transformation|GetActorLocation (Variables|Default|GetCombatTarget)))))
    (:then_1
      (bind _returnvalue_2 (CallFunction|MakeDamageSpec))
      (Game|SpawnActorfromClass (Variables|/Script/CardGame.CgCardData|GetProjectileClass (.CardData (Utilities|Struct|BreakCgCardDefinition (Variables|Default|GetCardDefinition)))) (Math|Transform|MakeTransform (LocalVariables|GetSpawnLocation) (LocalVariables|GetSpawnRotation)) "AlwaysSpawn" "MultiplyWithRoot" _returnvalue _returnvalue_2 (.AsPawn (Utilities|Casting|CastToPawn _returnvalue))))))

(fn MakeDamageSpec
  (bind _returnvalue (Ability|GetAbilitySystemComponentfromActorInfo))
  (return (GameplayEffects|MakeOutgoingSpec _returnvalue "/Game/CardGame/Blueprints/GAS/Effects/GE_Damage.GE_Damage_C" 1.0 (GameplayEffects|MakeEffectContext _returnvalue))))