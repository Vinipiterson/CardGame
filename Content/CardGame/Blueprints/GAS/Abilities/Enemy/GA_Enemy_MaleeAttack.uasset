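; Gameplay ability for an enemy melee attack, configured by the avatar's card definition.
; On activation it sets the facing warp target to the combat target and plays a random attack montage.
; Attack gameplay events trigger a sphere overlap-style trace at the card's attack socket.
; Hit combat actors outside the avatar's team receive a damage GameplayEffect, optionally limited to one hit per activation, and the ability ends with the montage.
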(event Ability|EventActivateAbility
  (bind _carddefinition (Variables|Default|GetCardDefinition))
  (bind _carddata (Utilities|Struct|BreakCgCardDefinition _carddefinition))
  (bind _returnvalue (Class|CgCardData|GetRandomAttackMontage _carddata))
  (bind _returnvalue_2 (Ability|CommitAbility))
  (if _returnvalue_2
    (Variables|Default|SetDamageApplied false)
    (CallFunction|UpdateFacingWarpTarget)
    (CallFunction|UpdateTeamTag)
    (CallFunction|UpdateCardDefinition)
    (Utilities|IsValid _returnvalue
      (:Is%20Valid
        (|PlayMontageandWaitProxy "None" _returnvalue 1.0 "None" false 1.0 0.0 false
          (:then
            (Ability|Tasks|WaitGameplayEvent "(TagName=\"CardGame.Ability.Event.Attack\")" 0
              (:EventReceived
                (bind (_outhits _returnvalue_3) (CallFunction|MaleeTrace))
                (if _returnvalue_3
                  (for _array_element _outhits
                    (CallFunction|ApplyDamage (.HitActor (Collision|BreakHitResult _array_element))))))))
          (:OnCompleted
            (Ability|EndAbility :!label _label))
          (:OnInterrupted
            (goto _label))
          (:OnCancelled
            (goto _label)))))))

(fn ApplyDamage
  (params (Target :type Actor%20Object%20Reference))
  (if (Utilities|DoesObjectImplementInterface Target "/Script/CardGame.CgCombatInterface")
    (bind _returnvalue (Class|CgCombatInterface|IsfromTeam(Message) Target (Variables|Default|GetTeamTag)))
    (if (not _returnvalue)
      (if (not (and (Variables|/Script/CardGame.CgCardData|GetbMaleeSingleHit (.CardData (Utilities|Struct|BreakCgCardDefinition (Variables|Default|GetCardDefinition)))) (Variables|Default|GetDamageApplied)))
        (Utilities|IsValid (Ability|GetAbilitySystemComponent Target)
          (:Is%20Valid
            (GameplayEffects|ApplyGameplayEffectSpecToSelf (Ability|GetAbilitySystemComponent Target) (Ability|MakeOutgoingGameplayEffectSpec (Variables|Default|GetDamageGameplayEffect)))
            (Variables|Default|SetDamageApplied true)))))))

(fn UpdateFacingWarpTarget
  (bind _returnvalue (Class|CgCombatInterface|GetCombatTarget(Message) (Ability|GetAvatarActorfromActorInfo)))
  (Utilities|IsValid _returnvalue
    (:Is%20Valid
      (Class|CgCombatInterface|SetFacingWarpTargetLocation(Message) (Ability|GetAvatarActorfromActorInfo) (Transformation|GetActorLocation _returnvalue)))))

(fn UpdateTeamTag
  (bind _returnvalue (Class|CgCombatInterface|GetTeamTag(Message) (Ability|GetAvatarActorfromActorInfo)))
  (Variables|Default|SetTeamTag _returnvalue))

(fn UpdateCardDefinition
  (bind _returnvalue (Class|CgCombatInterface|GetCardDefinition(Message) (Ability|GetAvatarActorfromActorInfo)))
  (Variables|Default|SetCardDefinition _returnvalue))

(fn MaleeTrace
  (bind _returnvalue (Ability|GetAvatarActorfromActorInfo))
  (bind _carddefinition (Variables|Default|GetCardDefinition))
  (bind _carddata (Utilities|Struct|BreakCgCardDefinition _carddefinition))
  (bind _returnvalue_2 (Actor|GetComponentbyClass _returnvalue "/Script/Engine.SkeletalMeshComponent"))
  (bind _attacksocketname (Variables|/Script/CardGame.CgCardData|GetAttackSocketName _carddata))
  (bind _returnvalue_3 (Transformation|GetSocketLocation _returnvalue_2 _attacksocketname))
  (bind (_outhits _returnvalue_4) (Collision|MultiSphereTraceForObjects _returnvalue_3 _returnvalue_3 (Variables|/Script/CardGame.CgCardData|GetMaleeTraceRadius (.CardData (Utilities|Struct|BreakCgCardDefinition (Variables|Default|GetCardDefinition)))) (Utilities|Array|MakeArray "ObjectTypeQuery3" "ObjectTypeQuery1") false 0 "None"))
  (return _outhits _returnvalue_4))