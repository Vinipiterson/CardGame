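; Team-owned tower actor for the card game, with a health bar driven by its Ability System Component.
; After a short delay on BeginPlay, it asks player controller 0 about its TeamTag to decide whether it is local.
; That flag picks a blue or red mesh material and initializes the health bar widget.
; It then listens for attribute changes and destroys itself when the value drops to zero or below.
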(event EventBeginPlay
  (Utilities|FlowControl|Delay 0.2)
  (bind _returnvalue (Class|CgCombatInterface|IsfromTeam(Message) (Game|GetPlayerController 0) (Variables|Default|GetTeamTag)))
  (Variables|Default|SetIsLocalTower _returnvalue)
  (Utilities|FlowControl|Sequence
    (:then_0
      (CallFunction|UpdateVisual))
    (:then_1
      (bind _aswbp_cg_health_bar (Utilities|Casting|CastToWBP_Cg_HealthBar (UserInterface|GetWidget (Variables|Default|GetWidget))))
      (Default|InitializeHealthBar _aswbp_cg_health_bar (Variables|Default|GetIsLocalTower) (Variables|Default|GetASC))
      (bind _newvalue (Ability|Tasks|WaitForAttributeChanged 0 "(AttributeName=\"Health\",Attribute=/Script/CardGame.CgVitalAttributeSet:Health,AttributeOwner=\"/Script/CoreUObject.Class'/Script/CardGame.CgVitalAttributeSet'\")")
        (:Changed
          (if (<= _newvalue 0.0)
            (Actor|DestroyActor)))))))

(fn ConstructionScript)

(fn UpdateVisual
  (if (Variables|Default|GetIsLocalTower)
    (Rendering|Material|SetMaterial (Variables|Default|GetStaticMesh) 0 "/Engine/OpenWorldTemplate/LandscapeMaterial/MI_ProcGrid_DarkBlue.MI_ProcGrid_DarkBlue")
    (else
      (Rendering|Material|SetMaterial (Variables|Default|GetStaticMesh) 0 "/Engine/OpenWorldTemplate/LandscapeMaterial/MI_ProcGrid_Red.MI_ProcGrid_Red"))))