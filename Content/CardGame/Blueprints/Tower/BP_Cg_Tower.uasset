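; BP_Cg_Tower is a card game tower Blueprint with a health bar widget.
; Shortly after BeginPlay, it casts the first player controller to CgPlayerController and its Widget component's content to WBP_Cg_HealthBar.
; It initializes the bar with the tower's Ability System Component, flagging it red when the local controller's Team differs from the tower's PlayerID.
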(event EventBeginPlay
  (Utilities|FlowControl|Delay 0.2)
  (bind _ascg_player_controller (Utilities|Casting|CastToCgPlayerController (Game|GetPlayerController 0)))
  (bind _aswbp_cg_health_bar (Utilities|Casting|CastToWBP_Cg_HealthBar (UserInterface|GetWidget (Variables|Default|GetWidget))))
  (Default|InitializeHealthBar _aswbp_cg_health_bar (!= (Variables|/Script/CardGame.CgPlayerController|GetTeam _ascg_player_controller) (Variables|Default|GetPlayerID)) (Variables|Default|GetASC)))

(fn ConstructionScript)