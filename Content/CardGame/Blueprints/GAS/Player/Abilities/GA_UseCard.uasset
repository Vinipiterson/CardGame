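; Gameplay ability that plays the player's current card, spawning the card's AI units at a targeted location.
; After committing, a target-data task supplies the hit location, then the player state provides the current card and discards it.
; Only the authority spawns the card's count of CgEnemy actors, passing the card definition and owner's team tag.
; Spawns are raised above the target, higher for air-terrain cards.
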(event Ability|EventActivateAbility
  (bind _returnvalue (Ability|CommitAbility))
  (if _returnvalue
    (bind _datahandle (|GetUseCardTargetData)
      (:ValidData
        (Variables|Default|SetTargetData (Ability|TargetData|GetHitResultfromTargetData _datahandle))
        (bind _asbp_cg_player_state (Utilities|Casting|CastToBP_Cg_PlayerState (Ability|GetOwningActorfromActorInfo))
          (:then
            (bind _output_get (Variables|Default|SetPS _asbp_cg_player_state))
            (Variables|Default|SetCardDefinition (Class|CgPlayerState|GetCurrentCard _output_get))
            (Class|CgPlayerState|DiscardCard (Variables|Default|GetPS))
            (if (Ability|HasAuthority (Ability|GetAvatarActorfromActorInfo))
              (for _index (range 1 (Variables|/Script/CardGame.CgCardData|GetNumToSpawn (.CardData (Utilities|Struct|BreakCgCardDefinition (Variables|Default|GetCardDefinition)))))
                (bind _returnvalue_2 (Class|CgCombatInterface|GetTeamTag(Message) (Ability|GetOwningActorfromActorInfo)))
                (Game|SpawnActorfromClass (.AsCg%20Enemy (Utilities|Casting|CastToCgEnemyClass (Variables|/Script/CardGame.CgCardData|GetAIClass (.CardData (Utilities|Struct|BreakCgCardDefinition (Variables|Default|GetCardDefinition)))))) (CallFunction|GetSpawnTransform) "AdjustIfPossibleButAlwaysSpawn" "MultiplyWithRoot" (Ability|GetOwningActorfromActorInfo) (Variables|Default|GetCardDefinition) _returnvalue_2 0))
              (Ability|EndAbility)
              (else
                (Ability|EndAbility))))
          (:CastFailed
            (Ability|CancelAbility)))))
    (else
      (Ability|CancelAbility))))

(fn GetSpawnTransform
  (return (Math|Transform|MakeTransform (+ (.Location (Collision|BreakHitResult (Variables|Default|GetTargetData))) (select (GameplayTags|MatchesTag (Variables|/Script/CardGame.CgCardData|GetTerrainTag (.CardData (Utilities|Struct|BreakCgCardDefinition (Variables|Default|GetCardDefinition)))) "(TagName=\"CardGame.Terrain.Air\")") "0.000000,0.000000,300.000000" "0.000000,0.000000,100.000000")))))