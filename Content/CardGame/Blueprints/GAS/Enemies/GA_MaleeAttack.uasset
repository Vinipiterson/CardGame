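; Gameplay Ability for an enemy melee attack, driven by the avatar's card definition.
; On activation it commits, plays a random melee montage from the card data and waits for an Attack gameplay event.
; That event sphere-traces at the card's mesh socket, damaging the first or every hit actor through a GAS effect with SetByCaller negated base damage.
; The ability ends when the montage completes, is interrupted or is cancelled.
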(event Ability|EventActivateAbility
  (bind _returnvalue (Ability|CommitAbility))
  (if _returnvalue
    (bind _returnvalue_2 (Class|CgCombatInterface|GetCardDefinition(Message) (Ability|GetAvatarActorfromActorInfo)))
    (bind _output_get (Variables|Default|SetCardDefinition _returnvalue_2))
    (Utilities|IsValid (Class|CgCardData|GetRandomMaleeMontage (.CardData (Utilities|Struct|BreakCgCardDefinition _output_get)))
      (:Is%20Valid
        (|PlayMontageandWaitProxy "None" (Class|CgCardData|GetRandomMaleeMontage (.CardData (Utilities|Struct|BreakCgCardDefinition _output_get))) 1.0 "None" false 1.0 0.0 false
          (:then
            (Ability|Tasks|WaitGameplayEvent "(TagName=\"CardGame.Ability.Event.Attack\")" 0
              (:EventReceived
                (bind (_outhits _returnvalue_3) (Collision|MultiSphereTraceByChannel (Transformation|GetSocketLocation (Actor|GetComponentbyClass (Ability|GetAvatarActorfromActorInfo) "/Script/Engine.SkeletalMeshComponent") (Variables|/Script/CardGame.CgCardData|GetMaleeSocketName (.CardData (Utilities|Struct|BreakCgCardDefinition (Variables|Default|GetCardDefinition))))) (Transformation|GetSocketLocation (Actor|GetComponentbyClass (Ability|GetAvatarActorfromActorInfo) "/Script/Engine.SkeletalMeshComponent") (Variables|/Script/CardGame.CgCardData|GetMaleeSocketName (.CardData (Utilities|Struct|BreakCgCardDefinition (Variables|Default|GetCardDefinition))))) (Variables|/Script/CardGame.CgCardData|GetMaleeTraceRadius (.CardData (Utilities|Struct|BreakCgCardDefinition (Variables|Default|GetCardDefinition)))) "TraceTypeQuery1" false 0 "ForDuration"))
                (if _returnvalue_3
                  (if (Variables|/Script/CardGame.CgCardData|GetbMaleeSingleHit (.CardData (Utilities|Struct|BreakCgCardDefinition (Variables|Default|GetCardDefinition))))
                    (CallFunction|ApplyDamage (.HitActor (Collision|BreakHitResult (Utilities|Array|Get(acopy) _outhits))))
                    (else
                      (for _array_element _outhits
                        (CallFunction|ApplyDamage (.HitActor (Collision|BreakHitResult _array_element))))))))))
          (:OnCompleted
            (Ability|EndAbility :!label _label))
          (:OnInterrupted
            (goto _label))
          (:OnCancelled
            (goto _label)))))))

(fn ApplyDamage
  (params (Target :type Actor%20Object%20Reference))
  (Utilities|IsValid (Ability|GetAbilitySystemComponent Target)
    (:Is%20Valid
      (bind _returnvalue (Ability|GameplayEffect|AssignTagSetbyCallerMagnitude (Ability|MakeOutgoingGameplayEffectSpec (Variables|Default|GetDamageGameplayEffect)) "(TagName=\"CardGame.SetByCaller.Damage\")" (* (Variables|/Script/CardGame.CgCardData|GetBaseDamage (.CardData (Utilities|Struct|BreakCgCardDefinition (Variables|Default|GetCardDefinition)))) -1.0)))
      (GameplayEffects|ApplyGameplayEffectSpecToSelf (Ability|GetAbilitySystemComponent Target) _returnvalue))))